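; BP_BlackHole is a spinning actor that swallows the pickable item props and ends the game once enough are collected.
; On overlap it casts the other actor through a chain of Ball, Scooter, Hat and Bag types, destroys any match and increments a shared counter.
; When the counter reaches four it quits the game, while Tick rotates the sphere a fixed amount every frame.
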(event `self.ReceiveBeginPlay`
  (set `self.Counter` 0))

(event `self.ReceiveActorBeginOverlap`
  (params (OtherActor :type "Actor Object Reference"))
  (bind _asbp_ball (cast `/Game/ItemPicking/BP_Ball` OtherActor)
    (:`then`
      (`self.K2_DestroyActor` _asbp_ball))
    (:`CastFailed`
      (bind _asbp_scooter (cast `/Game/ItemPicking/BP_Scooter` OtherActor)
        (:`then`
          (`self.K2_DestroyActor` _asbp_scooter))
        (:`CastFailed`
          (bind _asbp_hat (cast `/Game/ItemPicking/BP_Hat` OtherActor)
            (:`then`
              (`self.K2_DestroyActor` _asbp_hat))
            (:`CastFailed`
              (bind _asbp_bag (cast `/Game/ItemPicking/BP_Bag` OtherActor))
              (`self.K2_DestroyActor` _asbp_bag)))))))
  (bind _output_get (set `self.Counter` (+ (`self.Counter`) 1)))
  (if (== _output_get 4)
    (`KismetSystemLibrary.QuitGame` null "Quit")))

(event `self.ReceiveTick`
  (params (DeltaSeconds :type "Float (single-precision)"))
  (`SceneComponent.K2_AddLocalRotation` (`self.Sphere`) (struct :`Yaw` 1.0) false false))

(fn `UserConstructionScript`)