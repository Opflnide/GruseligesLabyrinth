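; BP_Lever is an interactive lever that opens and closes the first BP_Door found in the level.
; PullLever plays a sound and uses a FlipFlop to alternately hide the door's cube and disable its collision, or restore both.
; The PullUpAndDown timeline swings the lever's rotation forward or in reverse to match.
; A box trigger shows a text prompt while overlapped.
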(event `self.ReceiveBeginPlay`
  (bind _returnvalue (`GameplayStatics.GetActorOfClass` "/Game/Objects/BP_Door.BP_Door_C"))
  (set `self.Door` _returnvalue)
  (`SceneComponent.SetVisibility` (`self.TextRender`) false false))

(event `PullLever`
  (bind _door (`self.Door`))
  (bind _door_2 (`self.Door`))
  (`GameplayStatics.PlaySoundAtLocation` "/Engine/EditorSounds/GamePreview/EjectFromPlayer_Cue.EjectFromPlayer_Cue" (`self.K2_GetActorLocation`) (struct) 1.0 1.0 0.0 null null null null)
  (`/Engine/EditorBlueprintResources/StandardMacros.FlipFlop`
    (:`A`
      (`SceneComponent.SetVisibility` (`/Game/Objects/BP_Door.Cube` _door) false false)
      (`self.SetActorEnableCollision` _door false)
      (bind (_direction _newtrack_0) (`Timeline|Pull Up and Down` :!label _label)
        (:`Update`
          (`SceneComponent.K2_SetRelativeRotation` (`self.Lever`) (`KismetMathLibrary.RLerp` (struct :`Pitch` -40.0) (struct :`Pitch` -120.0) _newtrack_0) false false))))
    (:`B`
      (`SceneComponent.SetVisibility` (`/Game/Objects/BP_Door.Cube` _door_2) true false)
      (`self.SetActorEnableCollision` _door_2 true)
      (goto _label :!via `Reverse`))))

(event `self.Box.OnComponentBeginOverlap`
  (params (OverlappedComponent :type "PrimitiveComponent Object Reference") (OtherActor :type "Actor Object Reference") (OtherComp :type "PrimitiveComponent Object Reference") (OtherBodyIndex :type Integer) (bFromSweep :type Boolean) (SweepResult :type "HitResult Structure (by ref)"))
  (`SceneComponent.SetVisibility` (`self.TextRender`) true false))

(event `self.Box.OnComponentEndOverlap`
  (params (OverlappedComponent :type "PrimitiveComponent Object Reference") (OtherActor :type "Actor Object Reference") (OtherComp :type "PrimitiveComponent Object Reference") (OtherBodyIndex :type Integer))
  (`SceneComponent.SetVisibility` (`self.TextRender`) false false))

(fn `UserConstructionScript`)