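; Voice trumpet actor that endlessly rises, announces "Tubbytime" and sinks again, starting from BeginPlay.
; The RiseAndSink timeline nudges the mesh one unit per update, with IsFinished choosing up or down, alongside rising and sinking sounds.
; Once raised, a delayed loop plays the Tubbytime sound three times, then the timeline runs in reverse.
; When the reverse finishes, ResetAnimation restarts the cycle.
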(event `self.ReceiveBeginPlay`
  (bind _staticmesh (`self.StaticMesh`))
  (bind _returnvalue (`SceneComponent.K2_GetComponentLocation` _staticmesh))
  (bind _relativelocation (`SceneComponent.RelativeLocation` (`self.StaticMesh`)))
  (set `self.isFinished` false :!label _label)
  (`KismetSystemLibrary.Delay` 3.0)
  (`GameplayStatics.PlaySoundAtLocation` "/Game/Sounds/voice_trumpet_rising.voice_trumpet_rising" _relativelocation (struct) 0.3 1.0 0.0 null null null null)
  (`Timeline|Rise and Sink` :!label _label_2
    (:`Update`
      (if (`self.isFinished`)
        (`SceneComponent.K2_SetWorldLocation` _staticmesh (- _returnvalue (0.0 0.0 1.0)) false false)
        (else
          (`SceneComponent.K2_SetWorldLocation` _staticmesh (+ _returnvalue (0.0 0.0 1.0)) false false))))
    (:`Finished`
      (if (`self.isFinished`)
        (`self.Reset Animation`)
        (else
          (`KismetSystemLibrary.Delay` 3.7)
          (`/Game/CustomFunctions/CustomForLoop.ForLoopWithDelay` 0 2 1.66
            (:`Loop Body`
              (`GameplayStatics.PlaySoundAtLocation` "/Game/Sounds/tubbytime.tubbytime" _relativelocation (struct) 5.0 1.0 0.0 null null null null))
            (:`Completed`
              (`GameplayStatics.PlaySoundAtLocation` "/Game/Sounds/voice_trumpet_sinking.voice_trumpet_sinking" (0.0 0.0 0.0) (struct) 0.2 1.0 0.0 null null null null)
              (`KismetSystemLibrary.Delay` 1.0)
              (set `self.isFinished` true)
              (goto _label_2 :!via `ReverseFromEnd`))))))))

(event `Reset Animation`
  (goto _label))

(fn `UserConstructionScript`)