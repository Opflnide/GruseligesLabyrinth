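; Scooter actor that shows a floating text label while something overlaps its Box trigger.
; Box overlap begin and end toggle the TextRender, which starts hidden on BeginPlay.
; Every Tick, the Box moves to the StaticMesh's world location and the text follows above it.
; The text copies the player character mesh's rotation with yaw flipped 180 degrees.
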(event `self.ReceiveBeginPlay`
  (`SceneComponent.SetVisibility` (`self.TextRender`) false false))

(event `self.ReceiveTick`
  (params (DeltaSeconds :type "Float (single-precision)"))
  (bind _textrender (`self.TextRender`))
  (bind _textrender_2 (`self.TextRender`))
  (bind _returnvalue (`SceneComponent.K2_GetComponentLocation` (`self.StaticMesh`)))
  (bind (_returnvalue_roll _returnvalue_pitch _returnvalue_yaw) (`KismetMathLibrary.BreakRotator` (`SceneComponent.K2_GetComponentRotation` (`Character.Mesh` (`GameplayStatics.GetPlayerCharacter` 0)))))
  (`/Engine/EditorBlueprintResources/StandardMacros.IsValid` _textrender
    (:`Is Valid`
      (`SceneComponent.K2_SetWorldLocation` _textrender (+ _returnvalue (0.0 0.0 100.0)) false false)
      (`SceneComponent.K2_SetWorldLocation` (`self.Box`) _returnvalue false false)
      (`/Engine/EditorBlueprintResources/StandardMacros.IsValid` _textrender_2
        (:`Is Valid`
          (`SceneComponent.K2_SetWorldRotation` _textrender_2 (`KismetMathLibrary.MakeRotator` _returnvalue_roll _returnvalue_pitch (+ _returnvalue_yaw 180.0)) false false))))))

(event `self.Box.OnComponentBeginOverlap`
  (params (OverlappedComponent :type "PrimitiveComponent Object Reference") (OtherActor :type "Actor Object Reference") (OtherComp :type "PrimitiveComponent Object Reference") (OtherBodyIndex :type Integer) (bFromSweep :type Boolean) (SweepResult :type "HitResult Structure (by ref)"))
  (`SceneComponent.SetVisibility` (`self.TextRender`) true false))

(event `self.Box.OnComponentEndOverlap`
  (params (OverlappedComponent :type "PrimitiveComponent Object Reference") (OtherActor :type "Actor Object Reference") (OtherComp :type "PrimitiveComponent Object Reference") (OtherBodyIndex :type Integer))
  (`SceneComponent.SetVisibility` (`self.TextRender`) false false))

(fn `UserConstructionScript`)