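; BP_Tubby is a Teletubby-style enemy that roams the navmesh and chases pawns it sees.
; MoveAround loops AI moves to random reachable points, picking another on success or failure.
; PawnSensing sightings start a chase, with a DoOnce switching to the walking animation and higher speed.
; Each sighting restarts a retriggerable delay, which on expiry restores the waiting animation and slower speed, re-arms the sprint and resumes wandering.
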(event `self.ReceiveBeginPlay`
  (`SkeletalMeshComponent.PlayAnimation` (`self.Mesh`) "/Game/Items/Models/tetetubies_waiting_Anim.tetetubies_waiting_Anim" true)
  (`self.MoveAround`))

(event `MoveAround`
  (bind _randomlocation (`NavigationSystemV1.K2_GetRandomLocationInNavigableRadius` (`self.K2_GetActorLocation`) 4000.0 null null))
  (`|AIMoveTo` self _randomlocation null 10.0
    (:`OnSuccess`
      _)
    (:`OnFail`
      _))
  (`self.MoveAround`))

(event `self.PawnSensing.OnSeePawn`
  (params (Pawn :type "Pawn Object Reference"))
  (`|ExecutionSequence`
    (:`then_0`
      (`/Engine/EditorBlueprintResources/StandardMacros.DoOnce` false :!label _label
        (:`Completed`
          (`SkeletalMeshComponent.PlayAnimation` (`self.Mesh`) "/Game/Items/Models/tetetubies_walking4.tetetubies_walking4" true)
          (set `CharacterMovementComponent.MaxWalkSpeed` 400.0 (`self.CharacterMovement`)))))
    (:`then_1`
      (`|AIMoveTo` self (0.0 0.0 0.0) Pawn
        (:`then`
          (`KismetSystemLibrary.RetriggerableDelay` 5.0)
          (`SkeletalMeshComponent.PlayAnimation` (`self.Mesh`) "/Game/Items/Models/tetetubies_waiting_Anim.tetetubies_waiting_Anim" true)
          (set `CharacterMovementComponent.MaxWalkSpeed` 200.0 (`self.CharacterMovement`))
          (`self.CanSprintAgain`)
          (`self.MoveAround`))))))

(event `CanSprintAgain`
  (goto _label :!via `Reset`))

(fn `UserConstructionScript`)